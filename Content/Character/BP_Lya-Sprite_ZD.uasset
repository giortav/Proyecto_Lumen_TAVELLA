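; Paper2D side-scrolling player character Lya, with enhanced-input movement and jumping.
; On begin play it registers the input mapping context and sets the idle flipbook, with no later animation switching.
; Movement input runs along world X, and the sign of X acceleration sets controller yaw to face the character left or right.
; A light-collection event is a placeholder that only prints a debug string.
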(event `self.ReceiveBeginPlay`
  (bind _asplayer_controller (cast `PlayerController` (`self.GetController`)))
  (`EnhancedInputSubsystemInterface.AddMappingContext` (pcsubsystem `EnhancedInputLocalPlayerSubsystem` _asplayer_controller) "/Game/Inputs/MapingContext/IMC_PersonajeInputs.IMC_PersonajeInputs" 0 (struct))
  (`PaperFlipbookComponent.SetFlipbook` (`self.Sprite`) "/Game/Sprites/Reposo_.Reposo_"))

(event `EnhancedInput|/Game/Inputs/InputAction/IA_Movimiento`
  (params (ActionValue :type "Float (double-precision)") (ElapsedSeconds :type "Float (double-precision)") (TriggeredSeconds :type "Float (double-precision)") (InputAction :type "InputAction Object Reference" :default "/Game/Inputs/InputAction/IA_Movimiento.IA_Movimiento"))
  (bind _returnvalue_x (`KismetMathLibrary.BreakVector` (`CharacterMovementComponent.GetCurrentAcceleration` (`self.CharacterMovement`))))
  ;[0 0.8766 1] Movimiento personaje
  (:`Triggered`
    (`self.AddMovementInput` (1.0 0.0 0.0) ActionValue)
    ;[0 0.295 1] Rotación del personaje
    (`/Engine/EditorBlueprintResources/StandardMacros.CompareFloat` _returnvalue_x
      (:`>`
        (`Controller.SetControlRotation` (`self.GetController`) (`KismetMathLibrary.MakeRotator` 0.0)))
      (:`<`
        (`Controller.SetControlRotation` (`self.GetController`) (`KismetMathLibrary.MakeRotator` 0.0 0.0 180.0))))))

(event `EnhancedInput|/Game/Inputs/InputAction/IA_Saltar_`
  (params (ActionValue :type Boolean) (ElapsedSeconds :type "Float (double-precision)") (TriggeredSeconds :type "Float (double-precision)") (InputAction :type "InputAction Object Reference" :default "/Game/Inputs/InputAction/IA_Saltar_.IA_Saltar_"))
  ;[0.07967 0 1] Salto del personaje
  (:`Started`
    (`self.Jump`)))

(event `Event Recolectar Luces`
  ;[0 0.157 1] Recolectar luz
  (`KismetSystemLibrary.PrintString` "luz 1"))

(fn `UserConstructionScript`)